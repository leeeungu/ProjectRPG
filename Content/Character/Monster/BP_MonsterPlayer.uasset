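; BP_MonsterPlayer is a player-input Blueprint that attacks a nearby monster, apparently as a simple combat test.
; A Sphere overlap stores the overlapping C_MonsterBaseCharacter and its C_CounterComponent, and end overlap with any monster clears the monster reference.
; While that reference is valid, left click deals fixed damage and prints a debug string, and right click deals fixed stagger.
; The cached counter component is not used in these graphs.
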(event OnComponentBeginOverlap(Sphere)
  (params (OverlappedComponent :type Primitive%20Component%20Object%20Reference) (OtherActor :type Actor%20Object%20Reference) (OtherComp :type Primitive%20Component%20Object%20Reference) (OtherBodyIndex :type Integer) (bFromSweep :type Boolean) (SweepResult :type Hit%20Result%20Structure%20%28by%20ref%29))
  (bind _asc_monster_base_character (Utilities|Casting|CastToC_MonsterBaseCharacter OtherActor))
  (bind _output_get (Variables|Default|Setm_monster _asc_monster_base_character))
  (Variables|Default|Setm_counterCom (Actor|GetComponentbyClass _output_get "/Script/ProjectRPG.C_CounterComponent")))

(event OnComponentEndOverlap(Sphere)
  (params (OverlappedComponent :type Primitive%20Component%20Object%20Reference) (OtherActor :type Actor%20Object%20Reference) (OtherComp :type Primitive%20Component%20Object%20Reference) (OtherBodyIndex :type Integer))
  (Utilities|Casting|CastToC_MonsterBaseCharacter OtherActor)
  (Variables|Default|Setm_monster 0))

(event EventBeginPlay)

(event Collision|EventActorBeginOverlap
  (params (OtherActor :type Actor%20Object%20Reference)))

(event Input|MouseEvents|LeftMouseButton
  (params (Key :type Key%20Structure :default "None"))
  (bind _m_monster (Variables|Default|Getm_monster))
  (:Pressed
    (if (Utilities|IsValid _m_monster)
      (Class|CBaseCharacter|TakeDamageEvent _m_monster 1e+02)
      (Development|PrintString "attack"))))

(event Input|MouseEvents|RightMouseButton
  (params (Key :type Key%20Structure :default "None"))
  (bind _m_monster (Variables|Default|Getm_monster))
  (:Pressed
    (if (Utilities|IsValid _m_monster)
      (Class|CMonsterBaseCharacter|TakeStaggerEvent _m_monster 5e+01))))

(fn ConstructionScript)