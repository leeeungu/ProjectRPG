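; BP_StartPos is the entry point of a one-way teleport that moves BP_Player to a BP_EndPos actor.
; On BeginPlay it caches the location of the BP_EndPos found by GetActorOfClass.
; Overlapping the StartPos component starts a delay, then two back-to-back camera fades, the second replacing the first with a fade-out including audio.
; After another delay, SetActorLocation moves the player to the cached position.
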(event OnComponentBeginOverlap(StartPos)
  (params (OverlappedComponent :type Primitive%20Component%20Object%20Reference) (OtherActor :type Actor%20Object%20Reference) (OtherComp :type Primitive%20Component%20Object%20Reference) (OtherBodyIndex :type Integer) (bFromSweep :type Boolean) (SweepResult :type Hit%20Result%20Structure%20%28by%20ref%29))
  (bind _returnvalue (Game|GetPlayerController 0))
  (bind _playercameramanager (Variables|/Script/Engine.PlayerController|GetPlayerCameraManager _returnvalue))
  (bind _asbp_player (Utilities|Casting|CastToBP_Player OtherActor))
  (Utilities|FlowControl|Delay 3.0)
  (CameraFades|StartCameraFade :self _playercameramanager :FromAlpha 1.0 :Duration 3.0 :bShouldFadeAudio true)
  (CameraFades|StartCameraFade :self _playercameramanager :FromAlpha 0.0 :ToAlpha 1.0 :Duration 1.5 :bShouldFadeAudio true)
  (Utilities|FlowControl|Delay 2.0)
  (Transformation|SetActorLocation _asbp_player (Variables|Default|Getm_vTpPos) false false))

(event EventBeginPlay
  (bind _returnvalue (Actor|GetActorOfClass "/Game/Character/Monster/Teleport/BP_EndPos.BP_EndPos_C"))
  (Variables|Default|Setm_vTpPos (Transformation|GetActorLocation _returnvalue)))

(fn ConstructionScript)