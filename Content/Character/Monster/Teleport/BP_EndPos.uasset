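; BP_EndPos is a teleport end-position actor that starts the Lizardman boss encounter when it begins play.
; BeginPlay finds the BP_MonsterLizardman, has it set its target player and show its HP bar, and plays the boss room BGM.
; Its box destroys the actor when BP_Player leaves the overlap; the begin-overlap event only casts to the player and does nothing further.
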(event OnComponentBeginOverlap(Box)
  (params (OverlappedComponent :type Primitive%20Component%20Object%20Reference) (OtherActor :type Actor%20Object%20Reference) (OtherComp :type Primitive%20Component%20Object%20Reference) (OtherBodyIndex :type Integer) (bFromSweep :type Boolean) (SweepResult :type Hit%20Result%20Structure%20%28by%20ref%29))
  (Utilities|Casting|CastToBP_Player OtherActor))

(event OnComponentEndOverlap(Box)
  (params (OverlappedComponent :type Primitive%20Component%20Object%20Reference) (OtherActor :type Actor%20Object%20Reference) (OtherComp :type Primitive%20Component%20Object%20Reference) (OtherBodyIndex :type Integer))
  (Utilities|Casting|CastToBP_Player OtherActor)
  (Actor|DestroyActor))

(event EventBeginPlay
  (bind _returnvalue (Actor|GetActorOfClass "/Game/Character/Monster/MonsterBlueprints/Named/BP_MonsterLizardman.BP_MonsterLizardman_C"))
  (Variables|Default|SetBossMonster _returnvalue)
  (Default|SetTargetPlayer (Variables|Default|GetBossMonster))
  (Default|ViewHpBar (Variables|Default|GetBossMonster))
  (Audio|PlaySound2D "/Game/Audio/BGM/BossRoomBGM.BossRoomBGM" 1.0 1.0 0.0 0 0))

(fn ConstructionScript)