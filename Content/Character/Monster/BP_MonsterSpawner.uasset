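; BP_MonsterSpawner is a proximity-triggered spawner that creates a batch of random monsters when the player comes near.
; While active, Tick checks player distance, then spawns once, fires a spawn-complete dispatcher and deactivates itself.
; Each monster is picked from an array, given the player character as a blackboard object and bound to a death event.
; The death handler counts kills and prints the monster's name and running total.
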(event EventTick
  (params (DeltaSeconds :type Float%20%28single-precision%29))
  (if (Variables|Default|Getm_bIsActive)
    (Math|Float|CompareFloat (Math|Vector|VectorLength (- (Transformation|GetActorLocation self) (Transformation|GetActorLocation (Game|Player|GetPlayerPawn 0)))) 1e+03
      (:<
        (CallFunction|SpawnMonster)
        (Default|CallMonSpawnComplete)
        (bind _output_get (Variables|Default|Setm_bIsActive false))
        (Class|CMonsterSpawner|SetSpawnerActive _output_get)))))

(fn ConstructionScript)

(fn SpawnMonster
  (for _index (range 0 4)
    (bind _returnvalue (Game|SpawnActorfromClass (.OutItem (Utilities|Array|Random (Variables|Default|Getm_arrMonsters))) (Math|Transform|MakeTransform (Transformation|GetActorLocation)) "AdjustIfPossibleButAlwaysSpawn" "MultiplyWithRoot" 0 0))
    (AI|Components|Blackboard|SetValueasObject (AI|GetBlackboard (Pawn|GetController _returnvalue)) (LocalVariables|GetkeyName) (Game|GetPlayerCharacter 0))
    (EventDispatchers|BindEventtoMonMonsterDied _returnvalue (EventDispatchers|CreateEvent :!event OnMonsterDiedHandler))))

(fn OnMonsterDiedHandler
  (params (DeadMonster :type C%20Monster%20Base%20Character%20Object%20Reference))
  (bind _output_get (Variables|Default|Setm_nDeadCount (+ (Variables|Default|Getm_nDeadCount) 1)))
  (bind _output_get_2 (Variables|Default|Setm_deadMonsterName (Variables|/Script/ProjectRPG.C_MonsterBaseCharacter|Getm_strMonsterName DeadMonster)))
  (Development|PrintString (Utilities|String|ToString(Name) _output_get_2))
  (Development|PrintString (Utilities|String|ToString(Integer) _output_get)))