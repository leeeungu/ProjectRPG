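; BP_MonsterSpider is a normal monster Blueprint that sets up the spider's health and handles its death.
; BeginPlay fills HP from max HP, binds the death delegate and disables Tick.
; On death it plays a montage borrowed from the bear monster, stops AI, disables capsule collision and sets a short lifespan.
; Tick is re-enabled only then, sinking the corpse downward until it is destroyed.
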(event Custom|Dead
  (Animation|Montage|MontagePlay (Components|SkeletalMesh|GetAnimInstance (Variables|Character|GetMesh)) "/Game/Character/Monster/Animations/Montages/AM_MonsterBear_Dead_Montage.AM_MonsterBear_Dead_Montage" 1.0 "MontageLength" 0.0 true)
  (Class|CMonsterBaseCharacter|StopAi)
  (Collision|SetCollisionEnabled (Variables|Default|GetCapsuleComponent) "NoCollision")
  (Actor|Tick|SetActorTickEnabled true)
  (Actor|SetLifeSpan 2.0))

(event EventBeginPlay
  (Class|CBaseCharacter|SetHp (Variables|Default|Getm_fMaxHp))
  (EventDispatchers|BindEventtoMonDead (EventDispatchers|CreateEvent :!event Custom|Dead))
  (Actor|Tick|SetActorTickEnabled false))

(event EventTick
  (params (DeltaSeconds :type Float%20%28single-precision%29))
  (CallFunction|DeadandDestroy DeltaSeconds))

(fn ConstructionScript)

(fn DeadandDestroy
  (params (Delta :type Float%20%28double-precision%29))
  (Transformation|AddActorLocalOffset (Math|Vector|MakeVector 0.0 0.0 (* Delta -4e+01)) false false))