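; Lizardman boss monster Blueprint with phases, a stagger gimmick and a HUD health bar.
; On BeginPlay it fills HP, puts the player in the Blackboard as target and creates the health bar widget fed by itself and its stagger component.
; Damage passes HP to the phase and gimmick components; a phase change plays a montage, then adds an attack pattern and swaps the eye material.
; Tick prints HP after a delay.
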(event Custom|phaseChangeEvent
  (bind _returnvalue (Animation|Montage|MontagePlay (Components|SkeletalMesh|GetAnimInstance (Variables|Character|GetMesh)) "/Game/Character/Monster/Animations/Montages/Named/AM_Lizardman_phaseChange_Montage.AM_Lizardman_phaseChange_Montage" 1.0 "MontageLength" 0.0 true))
  (Utilities|FlowControl|Delay _returnvalue)
  (Utilities|Array|Add (Variables|Default|Getm_arrPatternList) (Variables|Default|GetNewPattern))
  (Rendering|Material|SetMaterial (Variables|Character|GetMesh) 1 "/Game/Lizardman_Berserker/Materials/M_Eyes_02.M_Eyes_02"))

(event EventBeginPlay
  (Class|CBaseCharacter|SetHp (Variables|Default|Getm_fMaxHp))
  (CallFunction|SetTargetPlayer)
  (EventDispatchers|BindEventtoMonPhaseChange (Variables|Default|GetC_Phase) (EventDispatchers|CreateEvent :!event Custom|phaseChangeEvent))
  (bind _returnvalue (UserInterface|CreateWidget "/Game/Character/Monster/UI/W_MonsterHpBar.W_MonsterHpBar_C" 0 self (Variables|Default|GetC_Stagger)))
  (UserInterface|Viewport|AddtoViewport _returnvalue 0))

(event EventTick
  (params (DeltaSeconds :type Float%20%28single-precision%29))
  (Utilities|FlowControl|Delay 4.0)
  (Development|PrintString (Utilities|String|ToString(Float) (Class|CBaseCharacter|GetHp))))

(fn ConstructionScript)

(fn SetTargetPlayer
  (AI|Components|Blackboard|SetValueasObject (AI|GetBlackboard (Pawn|GetController)) (Variables|Default|GetkeyName) (Game|GetPlayerCharacter 0)))

(fn TakeDamageEvent
  (params (fDamage :type Float%20%28single-precision%29))
  (bind _c_staggergimmick (Variables|Default|GetC_StaggerGimmick))
  (bind _returnvalue (|CallParentFunction fDamage))
  (if _returnvalue
    (Class|CPhaseComponent|PhaseChange (Variables|Default|GetC_Phase) (Variables|Default|Getm_fHp) (Variables|Default|Getm_fMaxHp))
    (bind _returnvalue_2 (Class|CGimmickComponent|CanGimmickStart _c_staggergimmick (Variables|Default|Getm_fHp) (Variables|Default|Getm_fMaxHp)))
    (if _returnvalue_2
      (Default|CallMonStaggerGimmickStart _c_staggergimmick)
      (return _returnvalue))
    (else
      (return _returnvalue))))