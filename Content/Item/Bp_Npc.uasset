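; Interactable NPC actor that acts as a store, opened and closed through searching and run/end event functions.
; On detection it caches the player's game window manager, and running it swaps the quick slot for inventory and store windows and shows its own store widget created at BeginPlay.
; While open, it borrows the player's camera onto its CameraPosition and disables controller tick; ending reverses both.
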(event EventBeginPlay
  (bind _returnvalue (UserInterface|CreateWidget "/Game/UI/Store/WBP_NpcStoreWidget.WBP_NpcStoreWidget_C" (Game|GetPlayerController 0) self))
  (Variables|Default|SetNPC _returnvalue))

(fn ConstructionScript)

(fn BeginSearchingEvent
  (params (pOther :type Actor%20Object%20Reference))
  (Utilities|FlowControl|Sequence
    (:then_0
      (Variables|Default|SetGameWidget (Actor|GetComponentbyClass (Game|GetInstigatorController pOther) "/Script/ProjectRPG.C_GameWindowManager")))
    (:then_1
      (Variables|Default|SetP%20Other pOther))
    (:then_2
      (return true))))

(fn EndSearchingEvent
  (params (pOther :type Actor%20Object%20Reference))
  (Utilities|FlowControl|Sequence
    (:then_1
      (Variables|Default|SetGameWidget 0)
      (Variables|Default|SetCameraComponent 0))
    (:then_2
      (return false))))

(fn RunEvent
  (params (pOther :type Actor%20Object%20Reference))
  (Utilities|FlowControl|Sequence
    (:then_0
      (if (not (Variables|Default|GetbOpen))
        (Variables|Default|GetGameWidget
          (:then
            (Utilities|FlowControl|Sequence
              (:then_0
                (Class|CGameWindowManager|AddWidgettoMain (Variables|Default|GetGameWidget) "E_Inventory"))
              (:then_1
                (Class|CGameWindowManager|AddWidgettoMain (Variables|Default|GetGameWidget) "E_Store"))
              (:then_2
                (Class|CGameWindowManager|RemoveWidgetfromMain (Variables|Default|GetGameWidget) "E_QuickSlot"))
              (:then_3
                (Actor|Tick|SetActorTickEnabled (Game|GetInstigatorController (Variables|Default|GetP%20Other))))
              (:then_4
                (bind _newparam (Class|BPICamera|GetCamera(Message) (Variables|Default|GetP%20Other)))
                (Variables|Default|SetCameraComponent _newparam)
                (Transformation|AttachComponentToComponent _newparam (Variables|Default|GetCameraPosition) "None" "KeepRelative" "KeepRelative" "KeepRelative" true)
                (UserInterface|Viewport|AddtoViewport (Variables|Default|GetNPC) 0))
              (:then_5
                (Variables|Default|SetbOpen true))))
          (:else))))
    (:then_1
      (return true))))

(fn EndEvent
  (Utilities|FlowControl|Sequence
    (:then_0
      (if (Variables|Default|GetbOpen)
        (Variables|Default|GetGameWidget
          (:then
            (Utilities|FlowControl|Sequence
              (:then_0
                (Class|CGameWindowManager|RemoveWidgetfromMain (Variables|Default|GetGameWidget) "E_Inventory"))
              (:then_1
                (Class|CGameWindowManager|RemoveWidgetfromMain (Variables|Default|GetGameWidget) "E_Store"))
              (:then_2
                (Class|CGameWindowManager|AddWidgettoMain (Variables|Default|GetGameWidget) "E_QuickSlot"))
              (:then_3
                (Class|BPICamera|ResetCamera(Message) (Variables|Default|GetP%20Other) (Variables|Default|GetCameraComponent))
                (Variables|Default|SetCameraComponent 0)
                (Widget|RemovefromParent (Variables|Default|GetNPC)))
              (:then_4
                (Actor|Tick|SetActorTickEnabled (Game|GetInstigatorController (Variables|Default|GetP%20Other)) true))
              (:then_5
                (Variables|Default|SetbOpen false))))
          (:else))))
    (:then_1
      (return true))))