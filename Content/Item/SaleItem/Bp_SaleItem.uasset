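; Bp_SaleItem is a usable item that sells for gold, adding its currency amount to the instigating player's currency component.
; It is usable only while the player's interaction target is a Bp_Npc with a store component.
; FindActor targets the instigator when a valid currency component exists, and ItemEffect pushes the gold using the ID from the item data subsystem.
; Both success and failure call the parent handler, then destroy the actor.
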(fn ConstructionScript)

(fn ItemEffect
  (Utilities|FlowControl|Sequence
    (:then_0
      (bind _asc_player (Utilities|Casting|CastToC_Player (Game|GetInstigator)))
      (bind _asc_player_controller (Utilities|Casting|CastToC_PlayerController (Pawn|GetController _asc_player)))
      (bind _returnvalue (Class|CCurrencyComponent|PushCurrency (Class|CPlayerController|GetCurrencyComponent _asc_player_controller) (Class|CItemDataSubsystem|GetCurrencyGoldItemID (Subsystems|GetCItemDataSubsystem)) (Variables|Default|GetN%20Currency%20Amount)))
      (return _returnvalue))
    (:then_1
      (return false))))

(fn FindActor
  (bind _returnvalue (Game|GetInstigator))
  (bind _asc_player (Utilities|Casting|CastToC_Player _returnvalue)
    (:then
      (bind _asc_player_controller (Utilities|Casting|CastToC_PlayerController (Pawn|GetController _asc_player))
        (:then
          (Utilities|IsValid (Class|CPlayerController|GetCurrencyComponent _asc_player_controller)
            (:Is%20Valid
              (return _returnvalue true))
            (:Is%20Not%20Valid
              _)))
        (:CastFailed
          _)))
    (:CastFailed
      _))
  (return 0 false))

(fn UseFail
  (bind _returnvalue (|CallParentFunction))
  (Actor|DestroyActor)
  (return _returnvalue))

(fn UseSuccess
  (bind _returnvalue (|CallParentFunction))
  (Actor|DestroyActor)
  (return _returnvalue))

(fn CheckItemUseable
  (Utilities|FlowControl|Sequence
    (:then_0
      (bind _asc_player (Utilities|Casting|CastToC_Player (Game|GetInstigator)))
      (bind _asbp_npc (Utilities|Casting|CastToBp_Npc (Class|CInteractionDetectorComponent|GetInteractionActor (Class|CPlayer|GetInteractionDetectComponent _asc_player))))
      (return (Utilities|IsValid (Actor|GetComponentbyClass _asbp_npc "/Script/ProjectRPG.C_StoreComponent"))))
    (:then_1
      (return false))))