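; Upgrade item Blueprint that raises the player's max HP when used.
; Its effect casts the instigator to C_Player and C_PlayerController, calls UpgradeMaxHP on MPEquipComponent with MaxHp, then plays a 2D use sound.
; Usability requires a valid equip component, while target finding checks the currency component and returns the instigator.
; Both use success and use failure call the parent, then destroy the item.
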(fn ConstructionScript)

(fn ItemEffect
  (Utilities|FlowControl|Sequence
    (:then_0
      (bind _asc_player (Utilities|Casting|CastToC_Player (Game|GetInstigator)))
      (bind _asc_player_controller (Utilities|Casting|CastToC_PlayerController (Pawn|GetController _asc_player)))
      (Class|CEquipComponent|UpgradeMaxHP (Variables|/Script/ProjectRPG.C_PlayerController|Getm_pEquipComponent _asc_player_controller) (Variables|Default|GetMaxHp))
      (Audio|PlaySound2D "/Game/Audio/Inventory/A_ItemUse.A_ItemUse" 1.0 1.0 0.0 0 0)
      (return true))
    (:then_1
      (return false))))

(fn FindActor
  (bind _returnvalue (Game|GetInstigator))
  (bind _asc_player (Utilities|Casting|CastToC_Player _returnvalue)
    (:then
      (bind _asc_player_controller (Utilities|Casting|CastToC_PlayerController (Pawn|GetController _asc_player))
        (:then
          (Utilities|IsValid (Class|CPlayerController|GetCurrencyComponent _asc_player_controller)
            (:Is%20Valid
              (return _returnvalue true))
            (:Is%20Not%20Valid
              _)))
        (:CastFailed
          _)))
    (:CastFailed
      _))
  (return 0 false))

(fn UseFail
  (bind _returnvalue (|CallParentFunction))
  (Actor|DestroyActor)
  (return _returnvalue))

(fn UseSuccess
  (bind _returnvalue (|CallParentFunction))
  (Actor|DestroyActor)
  (return _returnvalue))

(fn CheckItemUseable
  (Utilities|FlowControl|Sequence
    (:then_0
      (bind _asc_player (Utilities|Casting|CastToC_Player (Game|GetInstigator)))
      (bind _asc_player_controller (Utilities|Casting|CastToC_PlayerController (Pawn|GetController _asc_player)))
      (return (Utilities|IsValid (Class|CPlayerController|GetEquipComponent _asc_player_controller))))
    (:then_1
      (return false))))