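; Consumable upgrade item that raises the using player's attack power.
; ItemEffect reaches the equip component on the instigator's player controller, applies AttackValue, shows an on-screen Korean alert with the gain and plays a use sound.
; Usability requires that component to be valid, and FindActor targets the controller.
; The item destroys itself whether use succeeds or fails.
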(fn ConstructionScript)

(fn ItemEffect
  (bind _attackvalue (Variables|Default|GetAttackValue))
  (Utilities|FlowControl|Sequence
    (:then_0
      (bind _asc_player (Utilities|Casting|CastToC_Player (Game|GetInstigator)))
      (bind _asc_player_controller (Utilities|Casting|CastToC_PlayerController (Pawn|GetController _asc_player)))
      (Class|CEquipComponent|UpgradeAttack (Class|CPlayerController|GetEquipComponent _asc_player_controller) _attackvalue)
      (Class|CGameAlertSubsystem|PushAlertMessage (Subsystems|GetCGameAlertSubsystem) (Utilities|Struct|MakeS_GameAlertSubsystemConfig (Utilities|Text|FormatText "공격력이 {Value} 증가했습니다." _attackvalue) 2.0 true))
      (Audio|PlaySound2D "/Game/Audio/Inventory/A_ItemUse.A_ItemUse" 1.0 1.0 0.0 0 0)
      (return true))
    (:then_1
      (return false))))

(fn FindActor
  (bind _asc_player (Utilities|Casting|CastToC_Player (Game|GetInstigator))
    (:then
      (return (Pawn|GetController _asc_player) true))
    (:CastFailed
      (return 0 false))))

(fn UseFail
  (bind _returnvalue (|CallParentFunction))
  (Actor|DestroyActor)
  (return _returnvalue))

(fn UseSuccess
  (|CallParentFunction)
  (Actor|DestroyActor)
  (return true))

(fn CheckItemUseable
  (Utilities|FlowControl|Sequence
    (:then_0
      (bind _asc_player (Utilities|Casting|CastToC_Player (Game|GetInstigator)))
      (bind _asc_player_controller (Utilities|Casting|CastToC_PlayerController (Pawn|GetController _asc_player)))
      (return (Utilities|IsValid (Class|CPlayerController|GetEquipComponent _asc_player_controller))))
    (:then_1
      (return false))))