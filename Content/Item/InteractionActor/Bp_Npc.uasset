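; Interactable NPC actor that opens an NPC dialog screen with its own camera view for the player.
; Its interaction component tracks the overlapping player; interacting swaps the quick slot widget for the NPC widget and disables the controller's tick.
; The player's camera component is borrowed and attached to the NPC's CameraPosition.
; EndEvent restores widgets, camera and ticking, with an Open flag guarding both transitions.
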(event MonInteraction(m_pInteractionComponent)
  (params (pDetectedActor :type Actor%20Object%20Reference))
  (if (not (Variables|Default|GetbOpen))
    (Utilities|FlowControl|Sequence
      (:then_0
        (bind _asc_player_controller (Utilities|Casting|CastToC_PlayerController (Game|GetInstigatorController (Variables|Default|GetP%20Other))))
        (Variables|Default|SetGameWidget (Class|CPlayerController|GetGameWindowManager _asc_player_controller)))
      (:then_1
        (Variables|Default|GetGameWidget
          (:then
            (Utilities|FlowControl|Sequence
              (:then_0
                (Class|CGameWindowManager|RemoveWidgetfromMain (Variables|Default|GetGameWidget) "E_QuickSlot")
                (Class|CGameWindowManager|AddWidgettoMain (Variables|Default|GetGameWidget) "E_NPCWidget"))
              (:then_1
                (Actor|Tick|SetActorTickEnabled (Game|GetInstigatorController (Variables|Default|GetP%20Other))))
              (:then_2
                (bind _returnvalue (Class|CCameraInterface|GetCamera(Message) (Variables|Default|GetP%20Other)))
                (bind _output_get (Variables|Default|SetCameraComponent _returnvalue))
                (Utilities|IsValid _output_get
                  (:Is%20Valid
                    (Transformation|AttachComponentToComponent _output_get (Variables|Default|GetCameraPosition) "None" "KeepRelative" "KeepRelative" "KeepRelative" true))))
              (:then_3
                (Variables|Default|SetbOpen true))))
          (:else))))))

(event OnComponentBeginOverlap(m_pInteractionComponent)
  (params (OverlappedComponent :type Primitive%20Component%20Object%20Reference) (OtherActor :type Actor%20Object%20Reference) (OtherComp :type Primitive%20Component%20Object%20Reference) (OtherBodyIndex :type Integer) (bFromSweep :type Boolean) (SweepResult :type Hit%20Result%20Structure%20%28by%20ref%29))
  (bind _asc_player (Utilities|Casting|CastToC_Player OtherActor))
  (Variables|Default|SetP%20Other _asc_player))

(event OnComponentEndOverlap(m_pInteractionComponent)
  (params (OverlappedComponent :type Primitive%20Component%20Object%20Reference) (OtherActor :type Actor%20Object%20Reference) (OtherComp :type Primitive%20Component%20Object%20Reference) (OtherBodyIndex :type Integer))
  (Utilities|FlowControl|Sequence
    (:then_0
      (Variables|Default|SetGameWidget 0))
    (:then_1
      (Variables|Default|SetP%20Other 0))))

(fn ConstructionScript)

(fn EndEvent
  (if (Variables|Default|GetbOpen)
    (Variables|Default|GetGameWidget
      (:then
        (Utilities|FlowControl|Sequence
          (:then_0
            (Class|CGameWindowManager|AddWidgettoMain (Variables|Default|GetGameWidget) "E_QuickSlot")
            (Actor|Tick|SetActorTickEnabled (Variables|Default|GetP%20Other) true))
          (:then_1
            (Class|CCameraInterface|Reset(Message) (Variables|Default|GetP%20Other) (Variables|Default|GetCameraComponent))
            (Variables|Default|SetCameraComponent 0))
          (:then_2
            (Actor|Tick|SetActorTickEnabled (Game|GetInstigatorController (Variables|Default|GetP%20Other)) true))
          (:then_3
            (Variables|Default|SetbOpen false))
          (:then_4
            (Class|CGameWindowManager|RemoveWidgetfromMain (Variables|Default|GetGameWidget) "E_NPCWidget"))))
      (:else))))