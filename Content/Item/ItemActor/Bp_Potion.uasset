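; Healing potion item actor that runs UseItemActor on spawn and targets its instigator.
; Overrides the item-use hooks: ItemEffect adds a percentage of max HP, capped at max.
; CheckItemUseable, as wired, passes only at full HP, otherwise showing a "health full" alert.
; UseSuccess removes one item from the controller's inventory component, prints HP and destroys the actor; UseFail just destroys it.
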(event EventBeginPlay
  (Class|CItemActorBase|UseItemActor))

(fn ConstructionScript)

(fn FindActor
  (return (Game|GetInstigator) true))

(fn ItemEffect
  (bind _returnvalue (|CallParentFunction))
  (Utilities|FlowControl|Sequence
    (:then_0
      (bind _m_ptargetactor (Variables|Default|Getm_pTargetActor)
        (:then
          (bind _asc_base_character (Utilities|Casting|CastToC_BaseCharacter _m_ptargetactor))
          (bind _output_get (LocalVariables|SetHp (+ (Class|CBaseCharacter|GetHp _asc_base_character) (* (Class|CBaseCharacter|GetMaxHp _asc_base_character) (Variables|Default|GetHPPercent)))))
          (if (> _output_get (Class|CBaseCharacter|GetMaxHp _asc_base_character))
            (LocalVariables|SetHp (Class|CBaseCharacter|GetMaxHp _asc_base_character)))
          (Class|CBaseCharacter|SetHp _asc_base_character (LocalVariables|GetHp))
          (return true))
        (:else)))
    (:then_1
      (return _returnvalue))))

(fn UseFail
  (Actor|DestroyActor)
  (return true))

(fn UseSuccess
  (bind _returnvalue (Game|GetInstigator))
  (bind _returnvalue_2 (Game|GetInstigatorController _returnvalue))
  (bind _returnvalue_3 (Actor|GetComponentbyClass _returnvalue_2 "/Script/ProjectRPG.C_InventoryComponent"))
  (Utilities|IsValid _returnvalue_3
    (:Is%20Valid
      (bind _returnvalue_4 (Class|CInventoryComponent|RemoveItem _returnvalue_3 (Variables|Default|Getm_nItemID) 1))
      (if _returnvalue_4
        (bind _asc_base_character (Utilities|Casting|CastToC_BaseCharacter (Variables|Default|Getm_pTargetActor)))
        (Development|PrintString (Utilities|String|ToString(Float) (Class|CBaseCharacter|GetHp _asc_base_character)))
        (Actor|DestroyActor)
        (return true)
        (else
          _)))
    (:Is%20Not%20Valid
      _))
  (return false))

(fn CheckItemUseable
  (bind _asc_base_character (Utilities|Casting|CastToC_BaseCharacter (Variables|Default|Getm_pTargetActor))
    (:then
      (if (not (Math|Float|NearlyEqual(Float) (Class|CBaseCharacter|GetMaxHp _asc_base_character) (Class|CBaseCharacter|GetHp _asc_base_character) 1e-06))
        (Class|CGameAlertSubsystem|PushAlertMessage (Subsystems|GetCGameAlertSubsystem) (Utilities|Struct|MakeS_GameAlertSubsystemConfig "생명력이 득 찼습니다" 1.0 true))
        (return false)
        (else
          (return true))))
    (:CastFailed
      (return false))))