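; Throwable whirlwind grenade battle item that staggers monsters around the point under the player's cursor.
; On BeginPlay it checks that the target is in range, launches its mesh with a ballistic impulse solved from Life and gravity, and removes one item from inventory.
; Tick detonates it near the target, where a sphere trace staggers each monster once, then spawns a Niagara aura and destroys the actor.
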(event EventBeginPlay
  (bind _returnvalue (Game|GetInstigator))
  (bind _world_position (Variables|Default|GetWorld%20Position))
  (bind _life (Variables|Default|GetLife))
  (bind _returnvalue_2 (Transformation|GetActorLocation _returnvalue))
  (bind _returnvalue_3 (- _world_position _returnvalue_2))
  (bind _returnvalue_4 (/ _returnvalue_3 _life))
  (bind (_x _y) (Math|Vector|BreakVector _returnvalue_4))
  (Transformation|SetRelativeScale3D (Variables|Default|GetStaticMesh) "0.300000,0.300000,0.300000")
  (if (CallFunction|CheckItemUseable)
    (bind _output_get (Variables|Default|SetVelocity (Math|Vector|MakeVector _x _y (/ (+ (.Z (Math|Vector|BreakVector _returnvalue_3)) (* (* _life _life 0.5) 9.8e+02)) _life))))
    (Physics|AddImpulse (Variables|Default|GetStaticMesh) (* (Physics|GetMass (Variables|Default|GetStaticMesh)) _output_get) "None" false)
    (CallFunction|UseSuccess)
    (else
      (Actor|DestroyActor))))

(event EventTick
  (params (DeltaSeconds :type Float%20%28single-precision%29))
  (if (< (Math|Vector|Distance(Vector) (Transformation|GetActorLocation) (Variables|Default|GetWorld%20Position)) 1e+01)
    (CallFunction|ItemEffect)
    (Actor|Tick|SetActorTickEnabled false)
    (Actor|DestroyActor)
    (Niagara|SpawnSystematLocation "/Game/RPG_PayerVFX/AuraVFX/Fx/NS_Anime_Aura_1.NS_Anime_Aura_1" (Transformation|GetActorLocation))))

(fn ConstructionScript)

(fn FindActor
  (return 0 true))

(fn ItemEffect
  (bind _returnvalue (Transformation|GetActorLocation))
  (bind _returnvalue_2 (|CallParentFunction))
  (Utilities|FlowControl|Sequence
    (:then_0
      (bind (_outhits _returnvalue_3) (Collision|MultiSphereTraceForObjects _returnvalue _returnvalue 3e+02 (LocalVariables|GetTargetObject) false 0 "None"))
      (if _returnvalue_3
        (for _array_element _outhits
          (bind _asc_monster_base_character (Utilities|Casting|CastToC_MonsterBaseCharacter (.HitActor (Collision|BreakHitResult _array_element))))
          (if (not (Utilities|Set|Contains (LocalVariables|GetTargetActors) _asc_monster_base_character))
            (Class|CMonsterBaseCharacter|TakeStaggerEvent _asc_monster_base_character (Variables|Default|GetStagger))
            (Utilities|Set|Add (LocalVariables|GetTargetActors) _asc_monster_base_character)
            (Development|PrintString "Hello")))
        (return true)))
    (:then_1
      (return _returnvalue_2))))

(fn UseFail
  (Actor|DestroyActor)
  (return true))

(fn UseSuccess
  (bind _returnvalue (Game|GetInstigator))
  (bind _returnvalue_2 (Game|GetInstigatorController _returnvalue))
  (bind _returnvalue_3 (Actor|GetComponentbyClass _returnvalue_2 "/Script/ProjectRPG.C_InventoryComponent"))
  (Utilities|FlowControl|Sequence
    (:then_0
      (Utilities|IsValid _returnvalue_3
        (:Is%20Valid
          (bind _returnvalue_4 (Class|CInventoryComponent|RemoveItem _returnvalue_3 (Variables|Default|Getm_nItemID) 1))
          (if _returnvalue_4
            (return true)))))
    (:then_1
      (Actor|DestroyActor)
      (return false))))

(fn CheckItemUseable
  (Utilities|FlowControl|Sequence
    (:then_0
      (bind _asplayer_controller (Utilities|Casting|CastToPlayerController (Game|GetInstigatorController)))
      (if (.ReturnValue (Game|Player|GetHitResultUnderCursorbyChannel _asplayer_controller "TraceTypeQuery1" true))
        (Variables|Default|SetWorld%20Position (.impactpoint (.HitResult (Game|Player|GetHitResultUnderCursorbyChannel _asplayer_controller "TraceTypeQuery1" true))))
        (return (< (Math|Vector|Distance(Vector) (Transformation|GetActorLocation (Game|GetInstigator)) (Variables|Default|GetWorld%20Position)) 5e+02))))
    (:then_1
      (Actor|DestroyActor)
      (return false))))