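; Attack ring equipment item that changes the wearing character's attack power.
; On equip it applies the attack effect using its equip value, and on unequip it calls the matching removal with the same value.
; Both events push a timed on-screen Korean alert through the game alert subsystem, reporting the amount attack rose or fell.
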(event EventUnEffectEquip
  (params (pCharacter :type C%20Base%20Character%20Object%20Reference))
  (bind _m_fequipvalue (Variables|Default|Getm_fEquipValue))
  (Class|CEquipEffectFunctionLibrary|UnEffectAttack pCharacter _m_fequipvalue)
  (Class|CGameAlertSubsystem|PushAlertMessage (Subsystems|GetCGameAlertSubsystem) (Utilities|Struct|MakeS_GameAlertSubsystemConfig (Utilities|Text|FormatText "공격력이 {Value} 감소했습니다." _m_fequipvalue) 2.0 true)))

(event EventEffectEquip
  (params (pCharacter :type C%20Base%20Character%20Object%20Reference))
  (bind _m_fequipvalue (Variables|Default|Getm_fEquipValue))
  (Class|CEquipEffectFunctionLibrary|EffectAttack pCharacter _m_fequipvalue)
  (Class|CGameAlertSubsystem|PushAlertMessage (Subsystems|GetCGameAlertSubsystem) (Utilities|Struct|MakeS_GameAlertSubsystemConfig (Utilities|Text|FormatText "공격력이 {Value} 증가했습니다." _m_fequipvalue) 2.0 true)))

(fn ConstructionScript)