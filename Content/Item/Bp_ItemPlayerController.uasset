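; Player controller for the item system, with debug keys for exercising inventory, currency and interaction.
; On BeginPlay it adds the default and item Enhanced Input mapping contexts, shows the mouse cursor and caches the possessed character, refreshing it on pawn changes.
; Numpad debug keys push test items into MPInventoryComponent and add or remove gold through MPCurrencyComponent.
; Debug key G runs the C_Player's InteractionDetectComponent interaction.
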(event Custom|OnPossessedPawnChanged_이벤트
  (params (OldPawn :type Pawn%20Object%20Reference) (NewPawn :type Pawn%20Object%20Reference))
  ;[1 1 1] BeginPlay
  (bind _asc_player (Utilities|Casting|CastToC_Player NewPawn)
    (:then
      (Variables|Default|SetPossessedCharacter _asc_player))
    (:CastFailed
      (Variables|Default|SetPossessedCharacter 0))))

(event EventBeginPlay
  ;[1 1 1] BeginPlay
  (Utilities|FlowControl|Sequence
    (:then_0
      (Input|AddMappingContext (PlayerController|LocalPlayerSubsystems|GetEnhancedInputLocalPlayerSubsystem) "/Game/ThirdPerson/Input/IMC_Default.IMC_Default" 0 "(bIgnoreAllPressedKeysUntilRelease=True,bForceImmediately=False,bNotifyUserSettings=False)")
      (Variables|Default|SetbShowMouseCursor true))
    (:then_3
      (bind _ascharacter (Utilities|Casting|CastToCharacter (Pawn|GetControlledPawn)))
      (Variables|Default|SetPossessedCharacter _ascharacter))
    (:then_4
      (EventDispatchers|AssignOnPossessedPawnChanged (delegate Custom|OnPossessedPawnChanged_이벤트)))
    (:then_5
      (Input|AddMappingContext (PlayerController|LocalPlayerSubsystems|GetEnhancedInputLocalPlayerSubsystem) "/Game/Item/ItemInput/IAC_Item.IAC_Item" 0 "(bIgnoreAllPressedKeysUntilRelease=True,bForceImmediately=False,bNotifyUserSettings=False)"))))

(event Input|KeyboardEvents|DebugKeyG
  (params (Key :type Key%20Structure :default "None") (ActionValue :type Input%20Action%20Value%20Structure))
  (:Pressed
    (bind _asc_player (Utilities|Casting|CastToC_Player (Variables|Default|GetPossessedCharacter)))
    (Class|CInteractionDetectorComponent|RunInteraction (Class|CPlayer|GetInteractionDetectComponent _asc_player))))

(event Input|KeyboardEvents|DebugKeyNumPadTwo
  (params (Key :type Key%20Structure :default "None") (ActionValue :type Input%20Action%20Value%20Structure))
  ;[1 1 1] PushItem
  (:Pressed
    (Class|CCurrencyComponent|PopCurrency (Variables|Default|Getm_pCurrencyComponent) (Class|CItemDataSubsystem|GetCurrencyGoldItemID (Subsystems|GetCItemDataSubsystem)) 200)))

(event Input|KeyboardEvents|DebugKeyNumPadThree
  (params (Key :type Key%20Structure :default "None") (ActionValue :type Input%20Action%20Value%20Structure))
  ;[1 1 1] PushItem
  (:Pressed
    (Class|CInventoryComponent|PushItem (Variables|Default|Getm_pInventoryComponent) 2 100)))

(event Input|KeyboardEvents|DebugKeyNumPadFour
  (params (Key :type Key%20Structure :default "None") (ActionValue :type Input%20Action%20Value%20Structure))
  ;[1 1 1] PushItem
  (:Pressed
    (Class|CInventoryComponent|PushItem (Variables|Default|Getm_pInventoryComponent) 3 100)))

(event Input|KeyboardEvents|DebugKeyNumPadSeven
  (params (Key :type Key%20Structure :default "None") (ActionValue :type Input%20Action%20Value%20Structure))
  ;[1 1 1] PushItem
  (:Pressed
    (Class|CInventoryComponent|PushItem (Variables|Default|Getm_pInventoryComponent) 9 1)))

(event Input|KeyboardEvents|DebugKeyNumPadOne
  (params (Key :type Key%20Structure :default "None") (ActionValue :type Input%20Action%20Value%20Structure))
  ;[1 1 1] PushItem
  (:Pressed
    (Class|CCurrencyComponent|PushCurrency (Variables|Default|Getm_pCurrencyComponent) (Class|CItemDataSubsystem|GetCurrencyGoldItemID (Subsystems|GetCItemDataSubsystem)) 540)))

(fn ConstructionScript)