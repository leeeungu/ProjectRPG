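; BP_DemoPlayerController is a demo player controller that provides debug hotkeys for testing inventory and currency.
; Numpad keys add or remove gold through MPCurrencyComponent, resolving the gold ID from CItemDataSubsystem.
; Other numpad keys push hardcoded item IDs and counts into MPInventoryComponent.
; On BeginPlay it creates a WBP_RestartPlayer widget and adds it to the viewport.
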(event EventBeginPlay
  (bind _returnvalue (UserInterface|CreateWidget "/Game/UI/PlayerActionBar/WBP_RestartPlayer.WBP_RestartPlayer_C" self))
  (UserInterface|Viewport|AddtoViewport _returnvalue 0))

(event Input|KeyboardEvents|DebugKeyNumPadTwo
  (params (Key :type Key%20Structure) (ActionValue :type Input%20Action%20Value%20Structure))
  ;[1 1 1] ItemTest
  (:Pressed
    (Class|CCurrencyComponent|PopCurrency (Variables|Default|Getm_pCurrencyComponent) (Class|CItemDataSubsystem|GetCurrencyGoldItemID (Subsystems|GetCItemDataSubsystem)) 200)))

(event Input|KeyboardEvents|DebugKeyNumPadFour
  (params (Key :type Key%20Structure) (ActionValue :type Input%20Action%20Value%20Structure))
  ;[1 1 1] ItemTest
  (:Pressed
    (Class|CInventoryComponent|PushItem (Variables|Default|Getm_pInventoryComponent) 3 100)))

(event Input|KeyboardEvents|DebugKeyNumPadThree
  (params (Key :type Key%20Structure) (ActionValue :type Input%20Action%20Value%20Structure))
  ;[1 1 1] ItemTest
  (:Pressed
    (Class|CInventoryComponent|PushItem (Variables|Default|Getm_pInventoryComponent) 2 100)))

(event Input|KeyboardEvents|DebugKeyNumPadOne
  (params (Key :type Key%20Structure) (ActionValue :type Input%20Action%20Value%20Structure))
  ;[1 1 1] ItemTest
  (:Pressed
    (Class|CCurrencyComponent|PushCurrency (Variables|Default|Getm_pCurrencyComponent) (Class|CItemDataSubsystem|GetCurrencyGoldItemID (Subsystems|GetCItemDataSubsystem)) 540)))

(event Input|KeyboardEvents|DebugKeyNumPadFive
  (params (Key :type Key%20Structure) (ActionValue :type Input%20Action%20Value%20Structure))
  ;[1 1 1] ItemTest
  (:Pressed
    (Class|CInventoryComponent|PushItem (Variables|Default|Getm_pInventoryComponent) 8 1)))

(fn ConstructionScript
  (|CallParentFunction))