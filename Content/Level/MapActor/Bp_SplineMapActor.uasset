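; Spline-driven map actor that deforms a chosen static mesh along an editable spline.
; Its construction script adds one spline mesh component per segment between neighbouring points, attached to the root with a configurable forward axis.
; Each piece takes local positions from its two points and uses their arrive tangents at both start and end.
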(fn ConstructionScript
  (Utilities|FlowControl|Sequence
    (:then_0
      (LocalVariables|SetTotalCount (- (Spline|GetNumberOfSplinePoints (Variables|Default|GetSpline)) 2)))
    (:then_1
      (for _index (range 0 (LocalVariables|GetTotalCount))
        (bind _returnvalue (AddComponent|AddSplineMeshComponent true))
        (SplineMesh|SetForwardAxis _returnvalue (Variables|Default|GetIn%20Forward%20Axis) true)
        (Components|StaticMesh|SetStaticMesh _returnvalue (Variables|Default|GetSplineMesh))
        (Transformation|AttachComponentToComponent _returnvalue (Variables|Default|GetDefaultSceneRoot) "None" "KeepRelative" "KeepRelative" "KeepRelative" true)
        (SplineMesh|SetStartandEnd _returnvalue (.position (Spline|GetSplinePointAt (Variables|Default|GetSpline) _index "Local")) (.arrivetangent (Spline|GetSplinePointAt (Variables|Default|GetSpline) _index "Local")) (.position (Spline|GetSplinePointAt (Variables|Default|GetSpline) (+ _index 1) "Local")) (.arrivetangent (Spline|GetSplinePointAt (Variables|Default|GetSpline) (+ _index 1) "Local")) true :!class /Script/Engine.SplineMeshComponent)))))