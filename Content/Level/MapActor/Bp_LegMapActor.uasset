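; Bp_LegMapActor is a level map actor that configures two child Bp_SplineMapActor pieces at construction.
; The construction script casts each child actor, multiplies that child's MeshCount by its own MeshCount, then calls SpawnStaticMesh on it.
; The event graph holds only placeholder events, so the actor adds no runtime logic of its own.
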(event EventBeginPlay
  (|CallParentFunction) ; 지금 이 노드는 비활성 상태입니다. \n핀을 끌어서 다른 노드를 연결하면 활성화됩니다.
)

(event Collision|EventActorBeginOverlap
  (params (OtherActor :type Actor%20Object%20Reference)))

(event EventTick
  (params (DeltaSeconds :type Float%20%28single-precision%29)))

(fn ConstructionScript
  (|CallParentFunction)
  (Utilities|FlowControl|Sequence
    (:then_0
      (bind _asbp_spline_map_actor (Utilities|Casting|CastToBp_SplineMapActor (Variables|/Script/Engine.ChildActorComponent|GetChildActor (Variables|Default|GetChildActor))))
      (Variables|/Game/Level/MapActor/Bp_SplineMapActor.Bp_SplineMapActor_C|SetMeshCount _asbp_spline_map_actor (* (Variables|Default|GetMeshCount) (Variables|/Game/Level/MapActor/Bp_SplineMapActor.Bp_SplineMapActor_C|GetMeshCount _asbp_spline_map_actor)))
      (Default|SpawnStaticMesh _asbp_spline_map_actor))
    (:then_1
      (bind _asbp_spline_map_actor_2 (Utilities|Casting|CastToBp_SplineMapActor (Variables|/Script/Engine.ChildActorComponent|GetChildActor (Variables|Default|GetChildActor1))))
      (Variables|/Game/Level/MapActor/Bp_SplineMapActor.Bp_SplineMapActor_C|SetMeshCount _asbp_spline_map_actor_2 (* (Variables|Default|GetMeshCount) (Variables|/Game/Level/MapActor/Bp_SplineMapActor.Bp_SplineMapActor_C|GetMeshCount _asbp_spline_map_actor_2)))
      (Default|SpawnStaticMesh _asbp_spline_map_actor_2))))