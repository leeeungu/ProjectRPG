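; Floor map actor that fills an editable box area with a grid of randomly varied static mesh tiles.
; The construction script sizes the box from BoundBox and derives row and column counts from the first mesh's scaled bounds.
; Nested loops add a StaticMeshComponent per cell, picking mesh and rotation at random from arrays.
; BeginPlay only prints a debug size ratio; other event graph sizing logic never runs.
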(event EventBeginPlay
  (Development|PrintString (Utilities|String|ToString(Vector) (/ (Variables|/Script/Engine.BoxComponent|GetBoxExtent (Variables|Default|GetBox)) (* (.Max (Utilities|Struct|BreakBox (StaticMesh|GetBoundingBox (Utilities|Array|Get(acopy) (Variables|Default|GetNew%20Mesh))))) (Variables|Default|GetMeshScale) 0.5))) true true "(R=0.000000,G=0.660000,B=1.000000,A=1.000000)" 102.0))

(fn ConstructionScript
  (bind _meshscale (Variables|Default|GetMeshScale))
  (bind _new_mesh (Variables|Default|GetNew%20Mesh))
  (bind _bound_box (Variables|Default|GetBound%20Box))
  (bind _bound_box_2 (Variables|Default|GetBound%20Box))
  (bind _output (Utilities|Array|Get(acopy) _new_mesh))
  (bind _returnvalue (* _bound_box -1.0))
  (bind _returnvalue_2 (* _bound_box_2 2.0))
  (bind (_x _y) (Math|Vector|BreakVector _returnvalue_2))
  (bind _returnvalue_3 (StaticMesh|GetBoundingBox _output))
  (bind _max (Utilities|Struct|BreakBox _returnvalue_3))
  (bind _returnvalue_4 (* _max _meshscale))
  (Utilities|FlowControl|Sequence
    (:then_0
      (Components|Box|SetBoxExtent (Variables|Default|GetBox) _bound_box true)
      (LocalVariables|SetNewLocalVar (Math|Vector|MakeVector (.x _returnvalue) (.y _returnvalue) (.z (Transformation|GetActorLocation)))))
    (:then_1
      (if (Utilities|Array|IsNotEmpty _new_mesh)
        (Utilities|FlowControl|Sequence
          (:then_0
            (bind _output_get (LocalVariables|SetMeshOffset _returnvalue_4))
            (bind _output_get_2 (LocalVariables|SetNewLocalVar (Math|Vector|MakeVector (.X (Math|Vector|BreakVector (+ (LocalVariables|GetNewLocalVar) _output_get))) (.Y (Math|Vector|BreakVector (+ (LocalVariables|GetNewLocalVar) _output_get))) (* (.Z (Math|Vector|BreakVector _returnvalue_4)) -0.5))))
            (LocalVariables|SetMeshOffset (* (LocalVariables|GetMeshOffset) 2.0))
            (LocalVariables|SetSizeX (Math|Conversions|ToInteger(Byte) (Class|KismetMathLibrary|Round64 (/ _x (.x (LocalVariables|GetMeshOffset))))))
            (LocalVariables|SetSizeY (Math|Conversions|ToInteger(Byte) (Class|KismetMathLibrary|Round64 (/ _y (.y (LocalVariables|GetMeshOffset))))))
            (LocalVariables|SetStartPosition _output_get_2))
          (:then_1
            (for _index (range 1 (LocalVariables|GetSizeY))
              (for _index_2 (range 1 (LocalVariables|GetSizeX))
                (bind _returnvalue_5 (AddComponent|AddStaticMeshComponent true (Math|Transform|MakeTransform (LocalVariables|GetNewLocalVar) (.OutItem (Utilities|Array|Random (LocalVariables|GetNewLocalVar_0))) (Variables|Default|GetMeshScale))))
                (Components|StaticMesh|SetStaticMesh _returnvalue_5 (.OutItem (Utilities|Array|Random (Variables|Default|GetNew%20Mesh))))
                (Transformation|AttachComponentToComponent _returnvalue_5 (Variables|Transformation|GetRootComponent) "None" "KeepRelative" "KeepRelative" "KeepRelative" true)
                (LocalVariables|SetNewLocalVar (Math|Vector|MakeVector (+ (.x (LocalVariables|GetNewLocalVar)) (.x (LocalVariables|GetMeshOffset))) (.y (LocalVariables|GetNewLocalVar)) (.z (LocalVariables|GetNewLocalVar)))))
              (LocalVariables|SetNewLocalVar (Math|Vector|MakeVector (.x (LocalVariables|GetStartPosition)) (+ (.y (LocalVariables|GetNewLocalVar)) (.y (LocalVariables|GetMeshOffset))) (.z (LocalVariables|GetNewLocalVar)))))))))))