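; Linear slope map actor that procedurally builds a straight run of mesh pieces with supporting wall columns reaching down to the surface below.
; The construction script places static mesh components at multiples of Offset, repeated over the MeshCount range.
; At each piece's RightWall and LeftWall sockets, it traces downward on Visibility.
; On a hit, it stacks NewMesh copies below the socket, deriving their count from hit distance and mesh height.
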(fn ConstructionScript
  (bind _new_mesh (Variables|Default|GetNew%20Mesh))
  (bind _returnvalue (StaticMesh|GetBoundingBox _new_mesh))
  (Utilities|FlowControl|Sequence
    (:then_1
      (for _index (range 0 (Variables|Default|GetMeshCount))
        (bind _returnvalue_2 (AddComponent|AddStaticMeshComponent false (Math|Transform|MakeTransform (* _index (Variables|Default|GetOffset)) "0.000000,180.000000,0.000000" "1.000000,1.000000,1.000000")))
        (Transformation|AttachComponentToComponent _returnvalue_2 (Variables|Default|GetDefaultSceneRoot) "None" "KeepRelative" "KeepWorld" "KeepRelative" true)
        (Utilities|FlowControl|Sequence
          (:then_0
            (LocalVariables|SetNewLocalVar_2 "RightWall"))
          (:then_1
            (LocalVariables|SetNewLocalVar_2 "LeftWall")))
        (bind _outhit (Collision|LineTraceByChannel (Transformation|GetSocketLocation _returnvalue_2 (LocalVariables|GetNewLocalVar_2)) (+ (Transformation|GetSocketLocation _returnvalue_2 (LocalVariables|GetNewLocalVar_2)) (* (Math|Vector|VectorDown) 5e+03)) "TraceTypeQuery1" false (LocalVariables|GetNewLocalVar) "None" true "(R=1.000000,G=0.000000,B=0.000000,A=1.000000)" "(R=0.000000,G=1.000000,B=0.000000,A=1.000000)" 1.0))
        (if (.bBlockingHit (Collision|BreakHitResult _outhit))
          (bind _output_get (LocalVariables|SetNewLocalVar_0 (Math|Vector|Distance(Vector) (Transformation|GetSocketLocation _returnvalue_2 (LocalVariables|GetNewLocalVar_2)) (.ImpactPoint (Collision|BreakHitResult _outhit)))))
          (for _index_2 (range 1 (+ (Math|Float|Truncate (/ _output_get (- (.z (.max _returnvalue)) (.z (.min _returnvalue))))) 2))
            (bind _returnvalue_3 (AddComponent|AddStaticMeshComponent false))
            (Components|StaticMesh|SetStaticMesh _returnvalue_3 (Variables|Default|GetNew%20Mesh))
            (Transformation|AttachComponentToComponent _returnvalue_3 (Variables|Default|GetDefaultSceneRoot) "None" "KeepRelative" "KeepRelative" "KeepRelative" true)
            (Transformation|SetWorldLocation _returnvalue_3 (Math|Vector|MakeVector (.x (Transformation|GetSocketLocation _returnvalue_2 (LocalVariables|GetNewLocalVar_2))) (.y (Transformation|GetSocketLocation _returnvalue_2 (LocalVariables|GetNewLocalVar_2))) (- (.z (Transformation|GetSocketLocation _returnvalue_2 (LocalVariables|GetNewLocalVar_2))) (* _index_2 (- (.z (.Max (Components|StaticMesh|GetLocalBounds _returnvalue_3))) (.z (.Min (Components|StaticMesh|GetLocalBounds _returnvalue_3))))))) false false)
            (LocalVariables|SetNewLocalVar_0 (- (LocalVariables|GetNewLocalVar_0) 0.0))
            (Math|Integer|IncrementInt (LocalVariables|GetNewLocalVar_1))))))))