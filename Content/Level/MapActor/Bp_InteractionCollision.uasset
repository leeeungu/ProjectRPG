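; Map actor that toggles a Box collider according to the travel state of a nearby C_Player.
; Entering SearchCollision caches the player, subscribes to its travel component's change event and enables the Box; leaving unsubscribes and clears the reference.
; TypeChanged keeps the Box solid while the travel type is ENONE and disables its collision for any other type, also unbinding on ENONE if the player is outside the search volume.
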(event OnComponentEndOverlap(SearchCollision)
  (params (OverlappedComponent :type Primitive%20Component%20Object%20Reference) (OtherActor :type Actor%20Object%20Reference) (OtherComp :type Primitive%20Component%20Object%20Reference) (OtherBodyIndex :type Integer))
  (bind _asc_player (Utilities|Casting|CastToC_Player OtherActor))
  (bind _output_get (Variables|Default|SetAs%20C%20Player _asc_player))
  (EventDispatchers|UnbindEventfromMonTravelChanged (Class|CPlayer|GetTravelComponent _output_get) (EventDispatchers|CreateEvent :!event Custom|TypeChanged))
  (Variables|Default|SetAs%20C%20Player 0))

(event OnComponentBeginOverlap(SearchCollision)
  (params (OverlappedComponent :type Primitive%20Component%20Object%20Reference) (OtherActor :type Actor%20Object%20Reference) (OtherComp :type Primitive%20Component%20Object%20Reference) (OtherBodyIndex :type Integer) (bFromSweep :type Boolean) (SweepResult :type Hit%20Result%20Structure%20%28by%20ref%29))
  (bind _asc_player (Utilities|Casting|CastToC_Player OtherActor))
  (bind _output_get (Variables|Default|SetAs%20C%20Player _asc_player))
  (EventDispatchers|BindEventtoMonTravelChanged (Class|CPlayer|GetTravelComponent _output_get) (EventDispatchers|CreateEvent :!event Custom|TypeChanged))
  (Collision|SetCollisionEnabled (Variables|Default|GetBox) "QueryAndPhysics"))

(event Custom|TypeChanged
  (params (Pre :type E_TrabelType%20Enum :default "E_NONE") (Current :type E_TrabelType%20Enum :default "E_NONE"))
  (if (Utilities|Enum|Equal(Enum) Current "E_NONE")
    (Collision|SetCollisionEnabled (Variables|Default|GetBox) "QueryAndPhysics")
    (if (not (Collision|IsOverlappingActor (Variables|Default|GetSearchCollision) (Variables|Default|GetAs%20C%20Player) :!class /Script/Engine.PrimitiveComponent))
      (EventDispatchers|UnbindEventfromMonTravelChanged (Class|CPlayer|GetTravelComponent (Variables|Default|GetAs%20C%20Player)) (EventDispatchers|CreateEvent :!event Custom|TypeChanged)))
    (else
      (Collision|SetCollisionEnabled (Variables|Default|GetBox) "NoCollision"))))

(fn ConstructionScript)