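; Circle map actor that procedurally places a ring of randomized static meshes as level dressing.
; The construction script sets the sphere component's radius, then spawns mesh components at yaw steps around the actor, offset by that same radius.
; Each component draws its mesh, rotation and scale at random from arrays, attaches to the root and is stored in an array.
; BeginPlay is empty.
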(event EventBeginPlay)

(fn ConstructionScript
  (Utilities|FlowControl|Sequence
    (:then_0
      (Components|Sphere|SetSphereRadius (Variables|Default|GetSphere) (Variables|Default|GetIn%20Sphere%20Radius) true))
    (:then_1
      (if (Math|Boolean|ANDBoolean (Utilities|Array|IsNotEmpty (Variables|Default|GetNew%20Mesh)) (Utilities|Array|IsNotEmpty (Variables|Default|GetMeshRandomRotate)) (Utilities|Array|IsNotEmpty (Variables|Default|GetMeshRandomScale)))
        (for _index (range 0 (Variables|Default|GetMeshCount))
          (bind _output_get (LocalVariables|SetNewLocalVar (* (Math|Vector|RotateVector (Transformation|GetActorForwardVector) (Math|Rotator|MakeRotator 0.0 0.0 (* (/ (LocalVariables|GetNewLocalVar_0) (Variables|Default|GetMeshCount)) _index))) (Variables|Default|GetIn%20Sphere%20Radius))))
          (bind _returnvalue (AddComponent|AddStaticMeshComponent true (Math|Transform|MakeTransform _output_get (.OutItem (Utilities|Array|Random (Variables|Default|GetMeshRandomRotate))) (.OutItem (Utilities|Array|Random (Variables|Default|GetMeshRandomScale))))))
          (Components|StaticMesh|SetStaticMesh _returnvalue (.OutItem (Utilities|Array|Random (Variables|Default|GetNew%20Mesh))))
          (Transformation|AttachComponentToComponent _returnvalue (Variables|Transformation|GetRootComponent) "None" "KeepRelative" "KeepRelative" "KeepRelative" true)
          (Utilities|Array|Add (Variables|Default|GetMeshComponent) _returnvalue))))))