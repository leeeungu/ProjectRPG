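; Player controller that turns mouse and keyboard input into movement and skill commands for BP_TestPlayer, which it casts and caches at BeginPlay.
; Left-click events trace under the cursor to send the impact point to MoveToPosEvent, and also call PlainHit on the player's BPCSkill component.
; Q, W, E and R set a SkillNum enum and pass it to HowToUseSkill, while Space calls Period on the same component.
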(event EventBeginPlay
  (bind _asbp_test_player (Utilities|Casting|CastToBP_TestPlayer (Game|GetPlayerCharacter 0)))
  (Variables|Default|SetMyPlayer _asbp_test_player))

(event EventTick
  (params (DeltaSeconds :type Float%20%28single-precision%29)))

(event Input|MouseEvents|LeftMouseButton
  (params (Key :type Key%20Structure :default "None"))
  ;[1 1 1] PlainHit
  (:Pressed
    (Default|PlainHit (Variables|/Game/Player/BP_TestPlayer.BP_TestPlayer_C|GetBPC_Skill (Variables|Default|GetMyPlayer)))))

(event Input|KeyboardEvents|W
  (params (Key :type Key%20Structure :default "None"))
  ;[1 1 1] SkillInput
  (:Pressed
    (bind _output_get (Variables|Default|SetSkillNum "NewEnumerator1"))
    (Default|HowtoUseSkill (Variables|/Game/Player/BP_TestPlayer.BP_TestPlayer_C|GetBPC_Skill (Variables|Default|GetMyPlayer)) _output_get)))

(event Input|KeyboardEvents|Q
  (params (Key :type Key%20Structure :default "None"))
  ;[1 1 1] SkillInput
  (:Pressed
    (bind _output_get (Variables|Default|SetSkillNum "NewEnumerator0"))
    (Default|HowtoUseSkill (Variables|/Game/Player/BP_TestPlayer.BP_TestPlayer_C|GetBPC_Skill (Variables|Default|GetMyPlayer)) _output_get)))

(event Input|KeyboardEvents|SpaceBar
  (params (Key :type Key%20Structure :default "None"))
  ;[1 1 1] Period
  (:Pressed
    (Default|Period (Variables|/Game/Player/BP_TestPlayer.BP_TestPlayer_C|GetBPC_Skill (Variables|Default|GetMyPlayer)))))

(event Input|KeyboardEvents|R
  (params (Key :type Key%20Structure :default "None"))
  ;[1 1 1] SkillInput
  (:Pressed
    (bind _output_get (Variables|Default|SetSkillNum "NewEnumerator3"))
    (Default|HowtoUseSkill (Variables|/Game/Player/BP_TestPlayer.BP_TestPlayer_C|GetBPC_Skill (Variables|Default|GetMyPlayer)) _output_get)))

(event Input|KeyboardEvents|E
  (params (Key :type Key%20Structure :default "None"))
  ;[1 1 1] SkillInput
  (:Pressed
    (bind _output_get (Variables|Default|SetSkillNum "NewEnumerator2"))
    (Default|HowtoUseSkill (Variables|/Game/Player/BP_TestPlayer.BP_TestPlayer_C|GetBPC_Skill (Variables|Default|GetMyPlayer)) _output_get)))

(event Input|MouseEvents|LeftMouseButton
  (params (Key :type Key%20Structure :default "None"))
  (bind _returnvalue (Game|GetPlayerController 0))
  (bind (_hitresult _returnvalue_2) (Game|Player|GetHitResultUnderCursorbyChannel _returnvalue "TraceTypeQuery3" true))
  ;[1 1 1] Move
  (:Pressed
    (if _returnvalue_2
      (Default|MovetoPosEvent (Variables|Default|GetMyPlayer) (.impactpoint _hitresult)))))

(fn ConstructionScript)