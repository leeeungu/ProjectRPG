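; BPC_ComBat is a player combat component that runs a three-hit plain attack combo on the owning BP_TestPlayer.
; When input is enabled, each attack event plays the montage chosen by a combo counter, then increments it.
; The counter wraps after the third hit, and a retriggerable delay resets it when attacks stop coming, a placeholder marked for replacement by an input queue.
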(event Custom|PlainAttack%28Com%29_Event
  ;[1 1 1] 인풋이 가능할때 공격개시
  (if (Variables|Default|GetInputEnabled)
    (Animation|Montage|PlayMontage (Variables|/Script/Engine.Character|GetMesh (Variables|Default|GetMyPlayer)) (Utilities|Select :Index (Variables|Default|GetComboCounter) :Option%200 "/Game/Player/Skill/WukongAnimation/PlainAttack01_Montage.PlainAttack01_Montage" :Option%201 "/Game/Player/Skill/WukongAnimation/PlainAttack02_Montage.PlainAttack02_Montage" :Option%202 "/Game/Player/Skill/WukongAnimation/PlainAttack04_Montage.PlainAttack04_Montage")
      (:then
        (Math|Integer|IncrementInt (Variables|Default|GetComboCounter)
          (:%20%20
            (Utilities|FlowControl|Sequence
              (:then_0
                (if (== (Variables|Default|GetComboCounter) 3)
                  (Variables|Default|SetComboCounter 0)))
              (:then_1
                ;[1 1 1] InputQueue Test(change to Queue system)
                (Utilities|FlowControl|RetriggerableDelay 0.5)
                (Variables|Default|SetComboCounter 0)))))))))

(event EventBeginPlay
  (bind _asbp_test_player (Utilities|Casting|CastToBP_TestPlayer (Components|GetOwner)))
  (Variables|Default|SetMyPlayer _asbp_test_player))

(event EventCallSetInputEnabled
  (params (Enabled :type Boolean))
  (Variables|Default|SetInputEnabled Enabled))