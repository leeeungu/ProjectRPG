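; BPC_Skill is a player skill component that holds skill data and input key bindings.
; HowToUseSkill looks up the value bound to a skill key in the InputKeyDataSkill map.
; UpDataSkillInfo overwrites the damage percentage and cooldown of one SkillInfo array entry by index.
; CallDontMove, CallDontRotate and Period are empty stubs, and BeginPlay and Tick do nothing.
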(event EventBeginPlay)

(event EventTick
  (params (DeltaSeconds :type Float%20%28single-precision%29)))

(event EventCallDontMove
  (params (DontMove :type Boolean)))

(event EventCallDontRotate
  (params (DomtRoate :type Boolean)))

(fn HowtoUseSkill
  (params (SKillKey :type E_SkillKey%20Enum :default "NewEnumerator0"))
  (return (.Value (Utilities|Map|Find (Variables|Default|GetInputKeyData%28skill%29) SKillKey))))

(fn Period)

(fn UpDataSkillInfo
  (params (SkillIndex :type Integer) (NewDamagePercentage :type Float%20%28double-precision%29) (CoolTime :type Float%20%28double-precision%29))
  (bind _skillinfo (Variables|Default|GetSkillInfo))
  (bind _structout (Utilities|Struct|SetmembersinS_PlayerSkillInfo (Utilities|Array|Get(acopy) _skillinfo SkillIndex) NewDamagePercentage CoolTime))
  (Utilities|Array|SetArrayElem _skillinfo SkillIndex _structout))