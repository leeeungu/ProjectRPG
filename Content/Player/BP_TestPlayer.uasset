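; Test player actor that moves to a requested position, turns toward it, and triggers skills and plain attacks.
; Tick steps movement by capsule offsets and smooths yaw with a Lerp.
; Keys feed an input queue component, whose last index Tick routes to a skill montage or a placeholder item print, with a timed Delay standing in for notify-state input locking.
; Plain attacks are forwarded to the combat component.
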(event Custom|Attack
  (Animation|Montage|PlayMontage (Variables|Character|GetMesh) (.Animation (Utilities|Struct|BreakS_PlayerSkillInfo (Utilities|Array|Get(acopy) (Variables|/Game/Player/Skill/BPC_Skill.BPC_Skill_C|GetSkillInfo (Variables|Default|GetBPC_Skill)) (Variables|Default|GetSkillIndex))))))

(event Custom|MoveToPos_Event
  (params (NewParam :type Vector))
  (CallFunction|OnMovetoPos NewParam))

(event Custom|PlainAttack_Event
  ;[1 1 1] 2중이벤트호출(player controoler->player->combat)
  (CallFunction|DontMove false)
  (Default|PlainAttack(Com)Event (Variables|Default|GetBPC_ComBat)))

(event EventBeginPlay
  (bind _returnvalue (Transformation|GetActorRotation))
  (Variables|Default|SetCurrentRotation (.yaw _returnvalue))
  (Variables|Default|SetTargetRotation (.yaw _returnvalue)))

(event Collision|EventActorBeginOverlap
  (params (OtherActor :type Actor%20Object%20Reference)))

(event EventTick
  (params (DeltaSeconds :type Float%20%28single-precision%29))
  (CallFunction|Move DeltaSeconds)
  (CallFunction|Rotation DeltaSeconds)
  (bind _output_get (Variables|Default|SetCurrentRotation (Math|Float|Lerp (Variables|Default|GetCurrentRotation) (Variables|Default|GetTargetRotation) (* DeltaSeconds 2e+01))))
  (Transformation|SetActorRotation (Math|Rotator|MakeRotator 0.0 0.0 _output_get))
  (if (Variables|Default|GetIsInputEnabled)
    (bind _output_get_2 (Variables|Default|SetKeyIndexSetting (Class|CInputQueueComponant|OutputLastIndex (Variables|Default|GetC_InputQueueComponant) (Variables|Default|GetIsPull))))
    (CallFunction|InputEnabled _output_get_2 false)
    ;[1 1 1] Test 이제 애님몽타주에서 노티파이스테이트로 이두개 풀었다 잠궜다하면됨
    (Utilities|FlowControl|Delay 3.0)
    (Variables|Default|SetIsInputEnabled true)
    (Variables|Default|SetIsPull true)
    (Class|CInputQueueComponant|ClearList (Variables|Default|GetC_InputQueueComponant))))

(event Input|KeyboardEvents|F
  (params (Key :type Key%20Structure :default "None"))
  (:Pressed
    (CallFunction|Attack)))

(event Input|KeyboardEvents|B
  (params (Key :type Key%20Structure :default "None"))
  (bind _c_inputqueuecomponant (Variables|Default|GetC_InputQueueComponant))
  (:Pressed
    (Class|CInputQueueComponant|InputQueueList _c_inputqueuecomponant (Variables|Default|GetInput%20Key%20Data) (Variables|Default|GetIsAttacking))
    (Development|PrintString (Utilities|String|ToString(Integer) (Class|CInputQueueComponant|OutputLastIndex _c_inputqueuecomponant false)))))

(event Input|KeyboardEvents|G
  (params (Key :type Key%20Structure :default "None"))
  ;[1 1 1] 스킬을쓰면 바로 어태킹을 false바꿔서 어떤인풋이들어가든 0으로만듬
  (:Pressed
    (Variables|Default|SetKeyIndexSetting 5)
    (Variables|Default|SetIsAttacking false)
    (Utilities|FlowControl|Delay 5.0)
    (Variables|Default|SetIsAttacking true)))

(event Input|KeyboardEvents|V
  (params (Key :type Key%20Structure :default "None"))
  (bind _c_inputqueuecomponant (Variables|Default|GetC_InputQueueComponant))
  (:Pressed
    (Class|CInputQueueComponant|InputQueueList _c_inputqueuecomponant (Variables|Default|GetSkillIndex) (Variables|Default|GetIsAttacking))
    (Development|PrintString (Utilities|String|ToString(Integer) (Class|CInputQueueComponant|OutputLastIndex _c_inputqueuecomponant false)))))

(fn ConstructionScript)

(fn OnMovetoPos
  (params (NewPos :type Vector))
  (bind _capsulecomponent (Variables|Default|GetCapsuleComponent))
  (bind _capsulecomponent_2 (Variables|Default|GetCapsuleComponent))
  (bind _returnvalue (Transformation|GetWorldLocation _capsulecomponent))
  (bind _returnvalue_2 (- NewPos _returnvalue))
  (bind _returnvalue_3 (Math|Vector|VectorLength _returnvalue_2))
  (Variables|Default|SetRemainDist _returnvalue_3)
  (if (> _returnvalue_3 0.0)
    (bind _output_get (Variables|Default|SetMoveDir (Math|Vector|Normalize _returnvalue_2)))
    (Variables|Default|SetRemainAngle (Class|KismetMathLibrary|DegAcos (Math|Vector|DotProduct _output_get (Math|Vector|GetForwardVector _capsulecomponent_2))))
    (if (> (Math|Vector|DotProduct _output_get (Math|Vector|GetRightVector _capsulecomponent_2)) 0.0)
      (Variables|Default|SetRotDir 1.0)
      (else
        (Variables|Default|SetRotDir -1.0)))))

(fn Move
  (params (DeltaSeconds :type Float%20%28double-precision%29))
  (bind _capsulecomponent (Variables|Default|GetCapsuleComponent))
  (bind _movedir (Variables|Default|GetMoveDir))
  (bind _movespeed (Variables|Default|GetMoveSpeed))
  (bind _returnvalue (* DeltaSeconds _movespeed))
  (if (> (Variables|Default|GetRemainDist) 0.0)
    ;[1 1 1] Send to AnimBP of isMove(bool)
    (Variables|Default|SetIsMove true)
    (if (> _returnvalue (Variables|Default|GetRemainDist))
      (Transformation|AddWorldOffset _capsulecomponent (* _movedir (Variables|Default|GetRemainDist)) false false)
      (Variables|Default|SetRemainDist 0.0)
      (Variables|Default|SetIsMove false)
      (else
        (Transformation|AddWorldOffset _capsulecomponent (* _movedir _returnvalue) false false)
        (Variables|Default|SetRemainDist (- (Variables|Default|GetRemainDist) _returnvalue))))))

(fn Rotation
  (params (DeltaSeconds :type Float%20%28double-precision%29))
  (if (> (Variables|Default|GetRemainAngle) 0.0)
    (bind _output_get (Variables|Default|SetDeltaRotation (* DeltaSeconds 6e+02)))
    (if (> _output_get (Variables|Default|GetRemainAngle))
      (Variables|Default|SetDeltaRotation (Variables|Default|GetRemainAngle)))
    (Variables|Default|SetTargetRotation (+ (* (Variables|Default|GetRotDir) (Variables|Default|GetDeltaRotation)) (Variables|Default|GetTargetRotation)))
    (Variables|Default|SetRemainAngle (- (Variables|Default|GetRemainAngle) (Variables|Default|GetDeltaRotation)))))

(fn InputEnabled
  (params (HowKeyData :type Integer) (isEnabled :type Boolean))
  (Variables|Default|SetHowKeyData HowKeyData)
  ;[1 1 1] 0일땐 반환(즉 스킬데이터를 0로바꾸면 아무런 실행x)
  (if (== (Variables|Default|GetHowKeyData) 0)
    (return)
    (else
      (Variables|Default|SetIsPull false)
      ;[1 1 1] 1~8까지 데이터는 스킬함수호출
      (if (and (> (Variables|Default|GetHowKeyData) 0) (< (Variables|Default|GetHowKeyData) 9))
        ;[1 1 1] 애님노티파이스테이트로 들어가서 잠구고 attack함수 따로 제작
        (Variables|Default|SetIsInputEnabled false)
        (CallFunction|Attack)
        (return)
        (else
          ;[1 1 1] 10~19까지 데이터는 아이템함수호출
          (if (and (> (Variables|Default|GetHowKeyData) 9) (< (Variables|Default|GetHowKeyData) 20))
            (Development|PrintString "Item(Func)")
            (Variables|Default|SetKeyIndexSetting 0)
            (return)
            (else
              (Variables|Default|SetKeyIndexSetting 0)
              (return))))))))

(fn DontMove
  (params (DontMove :type Boolean))
  (if DontMove
    (Variables|Default|SetRemainDist 0.0)
    ;[1 1 1] animation(ABP_PLayer)
    (Variables|Default|SetIsMove false)
    (else
      (return))))