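; Quest actor that completes a purchase quest, by its name for armor, once the player obtains the required item quantities.
; On BeginPlay it destroys itself if the quest is finished, otherwise binds to the player inventory's push-item event and zeroes a counter per PurchaseItem key.
; Pushed items raise their counters, which are removed on reaching the target.
; An empty counter map clears the quest as succeeded through the QuestManager.
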(event Custom|PushItem
  (params (nItemID :type Integer) (nItemCount :type Integer))
  (bind _count (Variables|Default|GetCount))
  (bind (_value _returnvalue) (Utilities|Map|Find _count nItemID))
  (if (.ReturnValue (Utilities|Map|Find (Variables|Default|GetPurchaseItem) nItemID))
    (if _returnvalue
      (Utilities|Map|Add _count nItemID (+ _value nItemCount))
      (if (>= (.Value (Utilities|Map|Find (Variables|Default|GetCount) nItemID)) (.Value (Utilities|Map|Find (Variables|Default|GetPurchaseItem) nItemID)))
        (Utilities|Map|Remove (Variables|Default|GetCount) nItemID)
        (if (Utilities|Map|IsEmpty (Variables|Default|GetCount))
          (Class|CQuestManagerComponent|ClearQuest (Variables|Default|GetQuestManager) (Variables|Default|GetQuestAsset) true))))))

(event EventBeginPlay
  (if (Class|QuestAsset|GetFinishQuest (Variables|Default|GetQuestAsset))
    (Actor|DestroyActor)
    (else
      (bind _asc_player_controller (Utilities|Casting|CastToC_PlayerController (Game|GetPlayerController 0)))
      (Variables|Default|SetInventory (Class|CPlayerController|GetInventoryComponent _asc_player_controller))
      (Variables|Default|SetQuestManager (Class|CPlayerController|GetQuestManagerComponent _asc_player_controller))
      (EventDispatchers|BindEventtoMonPushItem (Class|CPlayerController|GetInventoryComponent _asc_player_controller) (EventDispatchers|CreateEvent :!event Custom|PushItem))
      (bind _keys (Utilities|Map|Keys (Variables|Default|GetPurchaseItem)))
      (for _array_element _keys
        (Utilities|Map|Add (Variables|Default|GetCount) _array_element 0)))))

(fn ConstructionScript)