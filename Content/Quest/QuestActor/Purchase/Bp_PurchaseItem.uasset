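; Quest actor that completes its assigned quest once the player acquires enough of a specified item.
; On BeginPlay it destroys itself if the quest is already finished, otherwise caches the player controller's inventory and quest manager and binds to the inventory's push-item delegate.
; Pushes of the matching item ID add to a running count, which clears the quest as succeeded through the quest manager at the required amount.
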(event Custom|PushItem
  (params (nItemID :type Integer) (nItemCount :type Integer))
  (if (== (Variables|Default|GetPurchaseItemID) nItemID)
    (Variables|Default|SetCount (+ (Variables|Default|GetCount) nItemCount))
    (if (>= (Variables|Default|GetCount) (Variables|Default|GetPurchaseItemCount))
      (Class|CQuestManagerComponent|ClearQuest (Variables|Default|GetQuestManager) (Variables|Default|GetQuestAsset) true))))

(event EventBeginPlay
  (if (Class|QuestAsset|GetFinishQuest (Variables|Default|GetQuestAsset))
    (Actor|DestroyActor)
    (else
      (bind _asc_player_controller (Utilities|Casting|CastToC_PlayerController (Game|GetPlayerController 0)))
      (Variables|Default|SetInventory (Class|CPlayerController|GetInventoryComponent _asc_player_controller))
      (Variables|Default|SetQuestManager (Class|CPlayerController|GetQuestManagerComponent _asc_player_controller))
      (EventDispatchers|BindEventtoMonPushItem (Class|CPlayerController|GetInventoryComponent _asc_player_controller) (EventDispatchers|CreateEvent :!event Custom|PushItem)))))

(fn ConstructionScript)