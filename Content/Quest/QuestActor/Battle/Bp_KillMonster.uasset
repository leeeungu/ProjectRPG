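; Quest actor for a kill-monsters objective that clears its quest once the expected number of monster deaths is reached.
; On BeginPlay it binds to the monster-died call of every BP_MonsterSpawner in the level and sets the target to a fixed five kills per spawner.
; UpdateDeadMonster counts deaths and, on reaching the target, calls ClearQuest as succeeded on the first player controller's quest manager component.
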(event Custom|UpdateDeadMonster
  (Math|Integer|IncrementInt (Variables|Default|GetCount)
    (:%20%20
      (if (== (Variables|Default|GetMaxCount) (Variables|Default|GetCount))
        (bind _asc_player_controller (Utilities|Casting|CastToC_PlayerController (Variables|Default|GetPlayer)))
        (Class|CQuestManagerComponent|ClearQuest (Class|CPlayerController|GetQuestManagerComponent _asc_player_controller) (Variables|Default|GetP%20Quest) true)))))

(event EventBeginPlay
  (bind _outactors (Actor|GetAllActorsOfClass "/Game/Character/Monster/BP_MonsterSpawner.BP_MonsterSpawner_C"))
  (Variables|Default|SetMaxCount (* (Utilities|Array|Length _outactors) 5))
  (for _array_element _outactors
    (EventDispatchers|BindEventtoMonMonsterDiedCall _array_element (EventDispatchers|CreateEvent :!event Custom|UpdateDeadMonster)))
  (Variables|Default|SetPlayer (Game|GetPlayerController 0)))

(fn ConstructionScript)