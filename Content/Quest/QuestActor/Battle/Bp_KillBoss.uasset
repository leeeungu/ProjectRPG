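; Quest actor for a boss-kill objective that completes a quest and shows the clear screen.
; On BeginPlay it finds a single monster character in the level by class and binds to its death event.
; The UpdateDead handler clears the quest as succeeded through the player controller's quest manager, then shows the clear widget and switches input to UI-only with the mouse locked.
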(event Custom|UpdateDead
  (bind _asc_player_controller (Utilities|Casting|CastToC_PlayerController (Variables|Default|GetPlayer)))
  (Class|CQuestManagerComponent|ClearQuest (Class|CPlayerController|GetQuestManagerComponent _asc_player_controller) (Variables|Default|GetP%20Quest) true)
  (bind _returnvalue (UserInterface|CreateWidget "/Game/UI/ChaosDungeon/WBP_ClearWidget.WBP_ClearWidget_C" (Variables|Default|GetPlayer)))
  (UserInterface|Viewport|AddtoViewport _returnvalue 0)
  (Widget|SetFocus _returnvalue)
  (Input|SetInputModeUIOnly (Variables|Default|GetPlayer) _returnvalue "LockAlways" false))

(event EventBeginPlay
  (Variables|Default|SetPlayer (Game|GetPlayerController 0))
  (bind _returnvalue (Actor|GetActorOfClass "/Script/ProjectRPG.C_MonsterBaseCharacter"))
  (Utilities|IsValid _returnvalue
    (:Is%20Valid
      (EventDispatchers|BindEventtoMonMonsterDied _returnvalue (EventDispatchers|CreateEvent :!event Custom|UpdateDead)))))

(fn ConstructionScript)