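; Quest actor that completes its QuestAsset when spline checkpoints are overlapped in order, and destroys itself if the quest is already finished.
; On BeginPlay it adds bound sphere colliders along the spline points and pushes the quest to the player controller's quest manager.
; Once the quest is accepted, overlapping the expected sphere advances an index; reaching the point count clears the quest as succeeded and destroys the actor.
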(event Custom|OverlapPlayer
  (params (OverlappedComponent :type Primitive%20Component%20Object%20Reference) (OtherActor :type Actor%20Object%20Reference) (OtherComp :type Primitive%20Component%20Object%20Reference) (OtherBodyIndex :type Integer) (bFromSweep :type Boolean) (SweepResult :type Hit%20Result%20Structure%20%28by%20ref%29))
  (if (Class|QuestAsset|GetQuestAccept (Variables|Default|GetQuest%20Asset))
    (if (== (Utilities|Array|Get(acopy) (Variables|Default|GetCollisions) (Variables|Default|GetIndex)) OverlappedComponent)
      (Math|Integer|IncrementInt (Variables|Default|GetIndex)
        (:%20%20
          (if (== (Spline|GetNumberOfSplinePoints (Variables|Default|GetSpline)) (Variables|Default|GetIndex))
            (Class|CQuestManagerComponent|ClearQuest (Class|CPlayerController|GetQuestManagerComponent (Variables|Default|GetAs%20C%20Player%20Controller)) (Variables|Default|GetQuest%20Asset) true)
            (Actor|DestroyActor)))))))

(event EventBeginPlay
  (bind _spline (Variables|Default|GetSpline))
  (|CallParentFunction)
  (if (Class|QuestAsset|GetFinishQuest (Variables|Default|GetQuest%20Asset))
    (Actor|DestroyActor)
    (else
      (bind _asc_player_controller (Utilities|Casting|CastToC_PlayerController (Game|GetPlayerController 0)))
      (Variables|Default|SetAs%20C%20Player%20Controller _asc_player_controller)
      (for _index (range 0 (Spline|GetNumberOfSplinePoints _spline))
        (bind _returnvalue (AddComponent|AddSphereComponent false (Math|Transform|MakeTransform (.position (Spline|GetSplinePointAt _spline _index "Local")) "0, 0, 0" "1.000000,1.000000,1.000000")))
        (Transformation|AttachComponentToComponent _returnvalue (Variables|Default|GetDefaultSceneRoot) "None" "KeepRelative" "KeepRelative" "KeepRelative" true)
        (Collision|BindEventtoOnComponentBeginOverlap _returnvalue (EventDispatchers|CreateEvent :!event Custom|OverlapPlayer))
        (Utilities|Array|Add (Variables|Default|GetCollisions) _returnvalue))
      (Class|CQuestManagerComponent|PushQuest (Class|CPlayerController|GetQuestManagerComponent (Variables|Default|GetAs%20C%20Player%20Controller)) (Variables|Default|GetQuest%20Asset)))))

(fn ConstructionScript)